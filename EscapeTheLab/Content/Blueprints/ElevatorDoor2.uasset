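; Two-panel elevator door that slides its left and right panels when something enters or leaves its Box trigger.
; Begin overlap moves both panels from their offsets to relative zero, and end overlap moves them back, with no filter on the overlapping actor.
; Each panel and direction has its own Timeline driving a location lerp, started with Play and never reset or reversed.
; DoorState is set immediately before each check, so it gates nothing.
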(event OnComponentBeginOverlap(Box)
  (params (OverlappedComponent :type Primitive%20Component%20Object%20Reference) (OtherActor :type Actor%20Object%20Reference) (OtherComp :type Primitive%20Component%20Object%20Reference) (OtherBodyIndex :type Integer) (bFromSweep :type Boolean) (SweepResult :type Hit%20Result%20Structure%20%28by%20ref%29))
  (Variables|Default|SetDoor_State true)
  (if (Variables|Default|GetDoor_State)
    (Utilities|FlowControl|Sequence
      (:then_0
        (bind _newtrack_0 (Timeline|Timeline_1 Play)
          (:Update
            (Transformation|SetRelativeLocation (Variables|Default|GetElevator_door_Right_door) (Math|Vector|Lerp(Vector) "376.315216,-0.000213,-2.832306" "0, 0, 0" _newtrack_0) false false))))
      (:then_1
        (bind _newtrack_0_2 (Timeline|Timeline_0 Play)
          (:Update
            (Transformation|SetRelativeLocation (Variables|Default|GetElevator_door_Left_door) (Math|Vector|Lerp(Vector) "225.458771,0.000000,0.000000" "0, 0, 0" _newtrack_0_2) false false)))))))

(event OnComponentEndOverlap(Box)
  (params (OverlappedComponent :type Primitive%20Component%20Object%20Reference) (OtherActor :type Actor%20Object%20Reference) (OtherComp :type Primitive%20Component%20Object%20Reference) (OtherBodyIndex :type Integer))
  (Variables|Default|SetDoor_State false)
  (if (not (Variables|Default|GetDoor_State))
    (Utilities|FlowControl|Sequence
      (:then_0
        (bind _newtrack_0 (Timeline|Timeline_3 Play)
          (:Update
            (Transformation|SetRelativeLocation (Variables|Default|GetElevator_door_Right_door) (Math|Vector|Lerp(Vector) "0, 0, 0" "376.315216,-0.000213,-2.832306" _newtrack_0) false false))))
      (:then_1
        (bind _newtrack_0_2 (Timeline|Timeline_2 Play)
          (:Update
            (Transformation|SetRelativeLocation (Variables|Default|GetElevator_door_Left_door) (Math|Vector|Lerp(Vector) "0, 0, 0" "225.458771, 0, 0" _newtrack_0_2) false false)))))))

(fn ConstructionScript)